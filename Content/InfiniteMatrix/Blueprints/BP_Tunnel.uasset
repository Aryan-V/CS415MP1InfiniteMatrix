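; BP_Tunnel is an endless-runner tunnel segment with a rotating wall obstacle that BP_Player must pass.
; RandomizeWall picks one of four hole meshes and a random roll, and Tick keeps the wall spinning.
; Hitting the wall damages the player, zeroes the segment's score increment and can trigger restart.
; The exit trigger has TunnelSpawner add a segment, destroys this one with its enemy and health pack, adds score and raises capped speed.
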(event `self.ReceiveTick`
  (params (DeltaSeconds :type "Float (single-precision)"))
  (`SceneComponent.K2_AddLocalRotation` (`self.WallMesh`) (`KismetMathLibrary.MakeRotator` (* DeltaSeconds (`self.RotateSpeed`))) false false))

(event `self.TriggerZone.OnComponentBeginOverlap`
  (params (OverlappedComponent :type "PrimitiveComponent Object Reference") (OtherActor :type "Actor Object Reference") (OtherComp :type "PrimitiveComponent Object Reference") (OtherBodyIndex :type Integer) (bFromSweep :type Boolean) (SweepResult :type "HitResult Structure (by ref)"))
  (bind _healthpack (`self.HealthPack`))
  (bind _enemy (`self.Enemy`))
  (bind _asbp_player (cast `/Game/InfiniteMatrix/Blueprints/BP_Player` OtherActor))
  (`/Game/InfiniteMatrix/Blueprints/BP_TunnelSpawner.SpawnTunnelAtSpawnPoint` (`self.TunnelSpawner`))
  (`self.K2_DestroyActor`)
  (`/Engine/EditorBlueprintResources/StandardMacros.IsValid` _enemy
    (:`Is Valid`
      (`self.K2_DestroyActor` _enemy))
    (:`Is Not Valid`
      _))
  (`/Engine/EditorBlueprintResources/StandardMacros.IsValid` _healthpack
    (:`Is Valid`
      (`self.K2_DestroyActor` _healthpack))
    (:`Is Not Valid`
      _))
  (bind _returnvalue (+ (`/Game/InfiniteMatrix/Blueprints/BP_Player.ScoreInt` _asbp_player) (`self.ToIncrementScore`)))
  (`/Game/InfiniteMatrix/UI/WBP_Score.Set Score` (`/Game/InfiniteMatrix/Blueprints/BP_Player.Score` _asbp_player) _returnvalue)
  (set `/Game/InfiniteMatrix/Blueprints/BP_Player.ScoreInt` _returnvalue _asbp_player)
  (bind _forwardspeed (`/Game/InfiniteMatrix/Blueprints/BP_Player.ForwardSpeed` _asbp_player))
  (if (<= _forwardspeed 4000.0)
    (set `self.ToIncrementScore` 10.0)
    (set `/Game/InfiniteMatrix/Blueprints/BP_Player.ForwardSpeed` (+ _forwardspeed 50.0) _asbp_player)))

(event `self.WallMesh.OnComponentBeginOverlap`
  (params (OverlappedComponent :type "PrimitiveComponent Object Reference") (OtherActor :type "Actor Object Reference") (OtherComp :type "PrimitiveComponent Object Reference") (OtherBodyIndex :type Integer) (bFromSweep :type Boolean) (SweepResult :type "HitResult Structure (by ref)"))
  (bind _asbp_player (cast `/Game/InfiniteMatrix/Blueprints/BP_Player` OtherActor))
  (bind _output_get (set `/Game/InfiniteMatrix/Blueprints/BP_Player.Health` (- (`/Game/InfiniteMatrix/Blueprints/BP_Player.Health` _asbp_player) 10.0) _asbp_player))
  (`/Game/InfiniteMatrix/UI/WBP_HealthBar.UpdateHealthUI` (`/Game/InfiniteMatrix/Blueprints/BP_Player.HealthBar` _asbp_player) _output_get)
  (set `self.ToIncrementScore` 0.0)
  (if (<= _output_get 0.0)
    (`/Game/InfiniteMatrix/Blueprints/BP_Player.DisplayRestart` _asbp_player)))

(fn `RandomizeWall`
  (`StaticMeshComponent.SetStaticMesh` (`self.WallMesh`) (select `int` (`KismetMathLibrary.RandomIntegerInRange` 0 3) :`0` "/Game/InfiniteMatrix/Meshes/SM_Hole_01.SM_Hole_01" :`1` "/Game/InfiniteMatrix/Meshes/SM_Hole_02.SM_Hole_02" :`2` "/Game/InfiniteMatrix/Meshes/SM_Hole_03.SM_Hole_03" :`3` "/Game/InfiniteMatrix/Meshes/SM_Hole_04.SM_Hole_04" :!type "StaticMesh Object Reference"))
  (`SceneComponent.K2_AddLocalRotation` (`self.WallMesh`) (`KismetMathLibrary.MakeRotator` (`KismetMathLibrary.Conv_IntToDouble` (`KismetMathLibrary.RandomIntegerInRange` 0 360))) false false))

(fn `UserConstructionScript`)